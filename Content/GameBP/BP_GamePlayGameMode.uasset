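; Gameplay game mode that runs the HUD, pause menu, key pickups and hero death/respawn flow.
; BeginPlay creates the widgets and binds hero dispatchers, so colored key pickups update the HUD and counter, only printing when all are collected.
; On death it hides the hero, possesses the first checkpoint found, stops enemies and shows the death menu.
; Restart repossesses the hero at that checkpoint and resets health, UI and all enemies.
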(event Custom|HeroIsDead
  ;[0.125 0.125 0.125] Hero is Dead
  (CallFunction|HideHeroChar)
  (CallFunction|PossesCheckpoint)
  (CallFunction|StopAllEnemies)
  (CallFunction|AddDeadMenuHidePlayerHUD)
  (EventDispatchers|AssignRestartfromCheckpoint (Variables|Default|GetW_DeadMenuRef) (delegate Custom|RestartFromCheckpoint_Event)))

(event Custom|PauseMenu
  (bind _w_pausemenuref (Variables|Default|GetW_PauseMenuRef))
  (bind _heroplayercontrollerref (Variables|Default|GetHeroPlayerControllerRef))
  ;[0.1354 0.1354 0.1354] Event PauseGame
  (Game|SetGamePaused true)
  (Widget|RemovefromParent (Variables|Default|GetW_HUDPlayerRef))
  (UserInterface|Viewport|AddtoViewport _w_pausemenuref 0)
  (Input|SetInputModeGameandUI _heroplayercontrollerref _w_pausemenuref "DoNotLock" true false)
  (Variables|/Script/Engine.PlayerController|SetbShowMouseCursor _heroplayercontrollerref true))

(event Custom|UnPauseMenu
  (bind _heroplayercontrollerref (Variables|Default|GetHeroPlayerControllerRef))
  ;[0.1198 0.1198 0.1198] Event Unpause Game
  (Game|SetGamePaused false)
  (Widget|RemovefromParent (Variables|Default|GetW_PauseMenuRef))
  (UserInterface|Viewport|AddtoViewport (Variables|Default|GetW_HUDPlayerRef) 0)
  (Input|SetInputModeGameOnly _heroplayercontrollerref false)
  (Variables|/Script/Engine.PlayerController|SetbShowMouseCursor _heroplayercontrollerref false))

(event Custom|RestartFromCheckpoint_Event
  ;[0.0625 0.0625 0.0625] Restart
  (Utilities|FlowControl|Sequence
    (:then_0
      (CallFunction|PossesHero)
      (CallFunction|UnHideHeroChar)
      (CallFunction|SetHeroPosition)
      (CallFunction|RestartHero))
    (:then_1
      (CallFunction|HideDeadMenuAddPlayerHUD0)
      (Default|UpdateUI (Variables|Default|GetW_HUDPlayerRef) (Variables|/Game/HeroChar/BP_Herochar.BP_Herochar_C|GetTotalHealth (Variables|Default|GetHeroCharRef))))
    (:then_2
      (CallFunction|RestartAllEnemies))))

(event Custom|PickKeyGreen_Event
  ;[0.1771 0.1771 0.1771] Assign Pickup
  (CallFunction|IncrementNumberKeysCheckTotal)
  (Default|ChangeKeyGreen (Variables|Default|GetW_HUDPlayerRef))
  (Variables|Default|SetisPickGreen true))

(event Custom|PickKeyPink_Event
  ;[0.1771 0.1771 0.1771] Assign Pickup
  (CallFunction|IncrementNumberKeysCheckTotal)
  (Default|ChangeKeyPink (Variables|Default|GetW_HUDPlayerRef))
  (Variables|Default|SetisPickPink true))

(event Custom|PkckKeyBlue_Event
  ;[0.1771 0.1771 0.1771] Assign Pickup
  (Default|ChangeKeyBlue (Variables|Default|GetW_HUDPlayerRef))
  (Variables|Default|SetisPickBlue true)
  (CallFunction|IncrementNumberKeysCheckTotal))

(event EventBeginPlay
  (Utilities|FlowControl|Sequence
    (:then_0
      ;[0.125 0.125 0.125] Get References
      (bind _asbp_herochar (Utilities|Casting|CastToBP_Herochar (Game|GetPlayerCharacter 0)))
      (Variables|Default|SetHeroCharRef _asbp_herochar)
      (bind _asbp_hero_controller (Utilities|Casting|CastToBP_HeroController (Game|GetPlayerController 0)))
      (Variables|Default|SetHeroPlayerControllerRef _asbp_hero_controller))
    (:then_1
      ;[0.07292 0.07292 0.07292] Creat HUD Player / Add to view Port
      (bind _returnvalue (UserInterface|CreateWidget "/Game/HUD/W_HUDPlayer.W_HUDPlayer_C" (Game|GetPlayerController 0)))
      (bind _output_get (Variables|Default|SetW_HUDPlayerRef _returnvalue))
      (UserInterface|Viewport|AddtoViewport _output_get 0)
      ;[0.08854 0.08854 0.08854] Create Pause Menu Widget
      (bind _returnvalue_2 (UserInterface|CreateWidget "/Game/HUD/W_MenuPause.W_MenuPause_C" (Game|GetPlayerController 0)))
      (Variables|Default|SetW_PauseMenuRef _returnvalue_2)
      ;[0.09375 0.09375 0.09375] Create Dead Menu
      (bind _returnvalue_3 (UserInterface|CreateWidget "/Game/HUD/W_MenuDead.W_MenuDead_C" (Game|GetPlayerController 0)))
      (Variables|Default|SetW_DeadMenuRef _returnvalue_3))
    (:then_2
      ;[0.1771 0.1771 0.1771] Assign Pickup
      (EventDispatchers|AssignPickKeyGreen (Variables|Default|GetHeroCharRef) (delegate Custom|PickKeyGreen_Event))
      (EventDispatchers|AssignPickKeyPink (Variables|Default|GetHeroCharRef) (delegate Custom|PickKeyPink_Event))
      (EventDispatchers|AssignPkckKeyBlue (Variables|Default|GetHeroCharRef) (delegate Custom|PkckKeyBlue_Event)))
    (:then_3
      ;[0.125 0.125 0.125] Hero is Dead
      (EventDispatchers|AssignHeroDead (Variables|Default|GetHeroCharRef) (delegate Custom|HeroIsDead)))))

(fn ConstructionScript)

(fn HideHeroChar
  (bind _herocharref (Variables|Default|GetHeroCharRef))
  (Rendering|SetActorHiddenInGame _herocharref true)
  (Rendering|SetActorHiddenInGame (Variables|/Game/HeroChar/BP_Herochar.BP_Herochar_C|GetGunRef _herocharref) true))

(fn UnHideHeroChar
  (bind _herocharref (Variables|Default|GetHeroCharRef))
  (Rendering|SetActorHiddenInGame _herocharref false)
  (Rendering|SetActorHiddenInGame (Variables|/Game/HeroChar/BP_Herochar.BP_Herochar_C|GetGunRef _herocharref) false))

(fn PossesCheckpoint
  (bind _outactors (Actor|GetAllActorsOfClass "/Game/Objects/Checkpoints/BP_Checkpoint.BP_Checkpoint_C"))
  (Pawn|Possess (Game|GetPlayerController 0) (Utilities|Array|Get(acopy) _outactors)))

(fn StopAllEnemies
  (bind _outactors (Actor|GetAllActorsOfClass "/Game/Enemy/BP_Enemy.BP_Enemy_C"))
  (for _array_element _outactors
    (Default|StopEnemyFire _array_element)))

(fn AddDeadMenuHidePlayerHUD
  (bind _w_deadmenuref (Variables|Default|GetW_DeadMenuRef))
  (UserInterface|Viewport|AddtoViewport _w_deadmenuref 0)
  (Widget|RemovefromParent (Variables|Default|GetW_HUDPlayerRef))
  (Input|SetInputModeUIOnly (Variables|Default|GetHeroPlayerControllerRef) _w_deadmenuref "DoNotLock" false)
  (Variables|/Script/Engine.PlayerController|SetbShowMouseCursor (Variables|Default|GetHeroPlayerControllerRef) true))

(fn PossesHero
  (Pawn|Possess (Game|GetPlayerController 0) (Variables|Default|GetHeroCharRef)))

(fn SetHeroPosition
  (bind _outactors (Actor|GetAllActorsOfClass "/Game/Objects/Checkpoints/BP_Checkpoint.BP_Checkpoint_C"))
  (Transformation|SetActorTransform (Variables|Default|GetHeroCharRef) (Transformation|GetActorTransform (Utilities|Array|Get(acopy) _outactors))))

(fn HideDeadMenuAddPlayerHUD0
  (UserInterface|Viewport|AddtoViewport (Variables|Default|GetW_HUDPlayerRef) 0)
  (Widget|RemovefromParent (Variables|Default|GetW_DeadMenuRef))
  (Input|SetInputModeGameOnly (Variables|Default|GetHeroPlayerControllerRef) false)
  (Variables|/Script/Engine.PlayerController|SetbShowMouseCursor (Variables|Default|GetHeroPlayerControllerRef) false))

(fn RestartHero
  (bind _herocharref (Variables|Default|GetHeroCharRef))
  (Variables|/Game/HeroChar/BP_Herochar.BP_Herochar_C|SetCurrentHealth _herocharref (Variables|/Game/HeroChar/BP_Herochar.BP_Herochar_C|GetTotalHealth _herocharref))
  (Variables|/Game/HeroChar/BP_Herochar.BP_Herochar_C|SetisDead _herocharref false)
  (Default|HeroRestartDeadState _herocharref))

(fn RestartAllEnemies
  (bind _outactors (Actor|GetAllActorsOfClass "/Game/Enemy/BP_Enemy.BP_Enemy_C"))
  (for _array_element _outactors
    (Variables|/Game/Enemy/BP_Enemy.BP_Enemy_C|SetisHeroOnSight _array_element false)
    (Variables|/Game/Enemy/BP_Enemy.BP_Enemy_C|SetisHeroHere _array_element false)
    (Default|RestartEnemy _array_element)
    (Variables|/Game/Enemy/BP_Enemy.BP_Enemy_C|SetEnemyHealth _array_element 1e+02)))

(fn IncrementNumberKeysCheckTotal
  (bind _result (Math|Integer|IncrementInt (Variables|Default|GetNumberKeysPickup))
    (:%20%20
      (if (== _result (Variables|Default|GetTotalKeys))
        (Development|PrintString "AllKeys")))))