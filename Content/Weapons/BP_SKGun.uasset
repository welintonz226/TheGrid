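; BP_SKGun is a hero weapon that fires BP_Projetil projectiles automatically while its trigger is active.
; On BeginPlay it caches the player's BP_Herochar.
; ActiveTrigger fires immediately and starts a looping timer on Fire at a rate set by ShootPerSecond, and DeactiveTrigger clears it.
; Each shot spawns a projectile at the hero's ArrowProjetil transform and plays a laser sound at the gun's location.
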(event Custom|ActiveTrigger
  ;[0.07292 0.07292 0.07292] Active Trigger / Deactive Trigger / Fire
  (CallFunction|Fire)
  (Utilities|Time|SetTimerbyFunctionName 0 "Fire" (/ 1.0 (Variables|Default|GetShootPerSecond)) true))

(event Custom|DeactiveTrigger
  ;[0.07292 0.07292 0.07292] Active Trigger / Deactive Trigger / Fire
  (Utilities|Time|ClearTimerbyFunctionName 0 "Fire"))

(event EventBeginPlay
  ;[0.1354 0.1354 0.1354] Get HeroChar -> HeroCharRef
  (bind _asbp_herochar (Utilities|Casting|CastToBP_Herochar (Game|GetPlayerCharacter 0)))
  (Variables|Default|SetHeroCharRef _asbp_herochar))

(fn ConstructionScript)

(fn Fire
  (Game|SpawnActorfromClass "/Game/Weapons/Projetil/BP_Projetil.BP_Projetil_C" (Transformation|GetWorldTransform (Variables|/Game/HeroChar/BP_Herochar.BP_Herochar_C|GetArrowProjetil (Variables|Default|GetHeroCharRef))) "Undefined" "MultiplyWithRoot" 0 0)
  (Audio|PlaySoundatLocation "/Game/Audio/421704__bolkmar__sfx-laser-shoot-02.421704__bolkmar__sfx-laser-shoot-02" (Transformation|GetActorLocation) "0, 0, 0" 1.0 1.0 0.0 0 0 0 0))