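; Key actor built from a core and two frame meshes, whose Pickup function returns its KeyColor.
; The construction script creates dynamic material instances for both frames, which ChangeMaterialParameters updates with a base color and emissive intensity.
; Timelines to spin the frames and bob the core exist but are never triggered, so the graph does not animate the key.
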(event EventBeginPlay)

(event Collision|EventActorBeginOverlap
  (params (OtherActor :type Actor%20Object%20Reference)))

(event EventTick
  (params (DeltaSeconds :type Float%20%28single-precision%29)))

(fn ConstructionScript
  (Utilities|FlowControl|Sequence
    (:then_0
      ;[0.06771 0.06771 0.06771] Create Dynamic Material Instance Frame1, Frame2
      (bind _returnvalue (Rendering|Material|CreateDynamicMaterialInstance (Variables|Default|GetFreame1) 1 "/Game/Objects/Floor/Materials/M_floorglow.M_floorglow" "None" :!class /Script/Engine.PrimitiveComponent))
      (Variables|Default|SetMaterialFrame1 _returnvalue))
    (:then_1
      (bind _returnvalue_2 (Rendering|Material|CreateDynamicMaterialInstance (Variables|Default|GetFreame2) 1 0 "None" :!class /Script/Engine.PrimitiveComponent))
      (Variables|Default|SetMaterialFrame2 _returnvalue_2))))

(fn Pickup
  (return (Variables|Default|GetKeyColor)))

(fn ChangeMaterialParameters
  (params (BaseColor :type Linear%20Color%20Structure) (EmissiveIntensity :type Float%20%28double-precision%29))
  (bind _materialframe1 (Variables|Default|GetMaterialFrame1))
  (bind _materialframe2 (Variables|Default|GetMaterialFrame2))
  (LocalVariables|SetLocalBaseColor BaseColor)
  (LocalVariables|SetLocalEmissiveIntensity EmissiveIntensity)
  (Utilities|FlowControl|Sequence
    (:then_0
      ;[0.1198 0.1198 0.1198] Change Frame1
      (Rendering|Material|SetScalarParameterValue _materialframe1 "EmissiveIntensity" (LocalVariables|GetLocalEmissiveIntensity) :!class /Script/Engine.MaterialInstanceDynamic)
      (Rendering|Material|SetVectorParameterValue _materialframe1 "BaseColor" (LocalVariables|GetLocalBaseColor) :!class /Script/Engine.MaterialInstanceDynamic))
    (:then_1
      ;[0.08854 0.08854 0.08854] Change Frame2
      (Rendering|Material|SetScalarParameterValue _materialframe2 "EmissiveIntensity" (LocalVariables|GetLocalEmissiveIntensity) :!class /Script/Engine.MaterialInstanceDynamic)
      (Rendering|Material|SetVectorParameterValue _materialframe2 "BaseColor" (LocalVariables|GetLocalBaseColor) :!class /Script/Engine.MaterialInstanceDynamic))))