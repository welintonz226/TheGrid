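; Interactable pink, green or blue totem that activates when the game mode's pick flag for its color is set.
; Construction creates a dynamic glow material and applies the totem's base color and idle emissive intensity.
; On Interact, TotemType selects the color check, which on success plays the AroAnimation ring timeline, switches to active emissive and spawns a BP_KeyFixo at the Arrow, tinted to match.
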(event Custom|ActiveTotemPink
  ;[0.1198 0.1198 0.1198] Active Totem Pink
  (if (Variables|/Game/GameBP/BP_GamePlayGameMode.BP_GamePlayGameMode_C|GetisPickPink (Variables|Default|GetGameModeRef))
    (Components|Timeline|PlayfromStart (Variables|Default|GetAroAnimation))
    (CallFunction|ChangeMaterialTotal (Variables|Default|GetBaseColor) (Variables|Default|GetEmissiveIntensityActive))
    (CallFunction|SpawnKey)))

(event Custom|ActiveTotemGreen
  ;[0.07812 0.07812 0.07812] ActiveTotemGreen
  (if (Variables|/Game/GameBP/BP_GamePlayGameMode.BP_GamePlayGameMode_C|GetisPickGreen (Variables|Default|GetGameModeRef))
    (Components|Timeline|PlayfromStart (Variables|Default|GetAroAnimation))
    (CallFunction|ChangeMaterialTotal (Variables|Default|GetBaseColor) (Variables|Default|GetEmissiveIntensityActive))
    (CallFunction|SpawnKey)))

(event Custom|ActiveTotemBlue
  ;[0.06771 0.06771 0.06771] ActiveTotemBlue
  (if (Variables|/Game/GameBP/BP_GamePlayGameMode.BP_GamePlayGameMode_C|GetisPickBlue (Variables|Default|GetGameModeRef))
    (Components|Timeline|PlayfromStart (Variables|Default|GetAroAnimation))
    (CallFunction|ChangeMaterialTotal (Variables|Default|GetBaseColor) (Variables|Default|GetEmissiveIntensityActive))
    (CallFunction|SpawnKey)))

(event EventBeginPlay
  ;[0.06771 0.06771 0.06771] Game Mode Reference
  (bind _asbp_game_play_game_mode (Utilities|Casting|CastToBP_GamePlayGameMode (Game|GetGameMode)))
  (Variables|Default|SetGameModeRef _asbp_game_play_game_mode))

(event EventInteract
  ;[0.09896 0.09896 0.09896] Event Interact  Interface
  (switch Utilities|FlowControl|Switch|SwitchonE_Keys (Variables|Default|GetTotemType)
    (:NewEnumerator0
      (CallFunction|ActiveTotemPink))
    (:NewEnumerator1
      (CallFunction|ActiveTotemGreen))
    (:NewEnumerator2
      (CallFunction|ActiveTotemBlue))))

(fn ConstructionScript
  (bind _returnvalue (Rendering|Material|CreateDynamicMaterialInstance (Variables|Default|GetTotem) 1 "/Game/StaticMeshs/Floor/Materials/MI_glowWhite.MI_glowWhite" "None" :!class /Script/Engine.PrimitiveComponent))
  (Variables|Default|SetTotemMaterial _returnvalue)
  (CallFunction|ChangeMaterialTotal (Variables|Default|GetBaseColor) (Variables|Default|GetEmissiveIntensity)))

(fn ChangeMaterialTotal
  (params (BaseColor :type Linear%20Color%20Structure) (Emissive :type Float%20%28double-precision%29))
  (bind _totemmaterial (Variables|Default|GetTotemMaterial))
  (Rendering|Material|SetVectorParameterValue _totemmaterial "BaseColor" BaseColor :!class /Script/Engine.MaterialInstanceDynamic)
  (Rendering|Material|SetScalarParameterValue _totemmaterial "EmissiveIntensity" Emissive :!class /Script/Engine.MaterialInstanceDynamic))

(fn SpawnKey
  (bind _returnvalue (Game|SpawnActorfromClass "/Game/Objects/Key/BP_KeyFixo.BP_KeyFixo_C" (Transformation|GetWorldTransform (Variables|Default|GetArrow)) "Undefined" "MultiplyWithRoot" 0 0))
  (Default|ChangeMaterialParameters _returnvalue (Variables|Default|GetBaseColor) (Variables|Default|GetEmissiveIntensityActive)))