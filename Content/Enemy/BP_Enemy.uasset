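; Drone enemy that bobs in place with a spinning antenna and shoots projectiles at the player.
; Timelines drive the randomized float and the antenna spin from BeginPlay.
; A capsule overlap or a hit alerts it; Tick then faces the player and starts a looping Fire timer through a DoOnce, controlled by StopEnemyFire and RestartEnemy.
; Hits reduce health with effects and sound, ending in an explosion and destruction.
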(event OnComponentBeginOverlap(Capsule)
  (params (OverlappedComponent :type Primitive%20Component%20Object%20Reference) (OtherActor :type Actor%20Object%20Reference) (OtherComp :type Primitive%20Component%20Object%20Reference) (OtherBodyIndex :type Integer) (bFromSweep :type Boolean) (SweepResult :type Hit%20Result%20Structure%20%28by%20ref%29))
  ;[0.05729 0.05729 0.05729] See HeroChar
  (Variables|Default|SetisHeroOnSight true)
  (Development|PrintString "Já te vi"))

(event Custom|StopEnemyFire
  (Utilities|Time|ClearTimerbyFunctionName 0 "Fire"))

(event Custom|RestartEnemy
  ;[0.09896 0.09896 0.09896] Rotate to direction Player / Call Timer By Function = Fire
  (Utilities|FlowControl|DoOnce false) ; enters at Reset
)

(event EventBeginPlay
  (Utilities|FlowControl|Sequence
    (:then_0
      ;[0.2292 0.2292 0.2292] Set Start  End Location / Set TimeLine Play Rate
      (bind _output_get (Variables|Default|SetStartLocation (Transformation|GetActorLocation)))
      (Variables|Default|SetEndLocation (+ _output_get (Math|Vector|MakeVector 0.0 0.0 (Math|Random|RandomFloatinRange 5e+01 1e+02))))
      (Components|Timeline|SetPlayRate (Variables|Default|GetDroneFloat) (Math|Random|RandomFloatinRange 1.0 2.0)))
    (:then_1
      ;[0.08333 0.08333 0.08333] Add Rotate Axe Z Antenna Drone
      (bind _rotatez (Timeline|RotateAntenna Play)
        (:Update
          (Transformation|AddLocalRotation (Variables|Default|GetAntennaMesh) (Math|Rotator|MakeRotator 0.0 0.0 _rotatez) false false)
          (Timeline|RotateAntenna Play))))
    (:then_2
      ;[0.1406 0.1406 0.1406] Drone Float
      (bind _alpha (Timeline|DroneFloat Play)
        (:Update
          (Transformation|SetActorLocation (Math|Vector|Lerp(Vector) (Variables|Default|GetStartLocation) (Variables|Default|GetEndLocation) _alpha) false false))))
    (:then_3
      ;[0.125 0.125 0.125] Referência do Player Character
      (bind _asbp_herochar (Utilities|Casting|CastToBP_Herochar (Game|GetPlayerCharacter 0)))
      (Variables|Default|SetHeroCharRef _asbp_herochar))))

(event Collision|EventHit
  (params (MyComp :type Primitive%20Component%20Object%20Reference) (Other :type Actor%20Object%20Reference) (OtherComp :type Primitive%20Component%20Object%20Reference) (bSelfMoved :type Boolean) (HitLocation :type Vector :default "0, 0, 0") (HitNormal :type Vector :default "0, 0, 0") (NormalImpulse :type Vector :default "0, 0, 0") (Hit :type Hit%20Result%20Structure%20%28by%20ref%29))
  (bind _returnvalue (Transformation|GetActorLocation))
  (bind _returnvalue_2 (Transformation|GetActorLocation))
  ;[0.08854 0.08854 0.08854] Event HIt - Damage and death Enemy
  (Variables|Default|SetisHeroHere true)
  (if (> (Variables|Default|GetEnemyHealth) (Variables|Default|GetDamageTaken))
    (Variables|Default|SetEnemyHealth (- (Variables|Default|GetEnemyHealth) (Variables|Default|GetDamageTaken)))
    (Niagara|SpawnSystematLocation "/Game/VFX/EnemyHit_System.EnemyHit_System" _returnvalue_2 "0, 0, 0" "0.100000,0.100000,0.100000")
    (Audio|PlaySoundatLocation "/Game/Audio/501104__evretro__8-bit-damage-sound_Cue.501104__evretro__8-bit-damage-sound_Cue" _returnvalue_2 "0, 0, 0" 1.0 1.0 0.0 0 0 0 0)
    (else
      (Effects|SpawnEmitteratLocation "/Game/StarterContent/Particles/P_Explosion.P_Explosion" _returnvalue)
      (Audio|PlaySoundatLocation "/Game/StarterContent/Audio/Explosion_Cue.Explosion_Cue" _returnvalue "0, 0, 0" 1.0 1.0 0.0 0 0 0 0)
      (Actor|DestroyActor))))

(event EventTick
  (params (DeltaSeconds :type Float%20%28single-precision%29))
  ;[0.09896 0.09896 0.09896] Rotate to direction Player / Call Timer By Function = Fire
  (if (or (Variables|Default|GetisHeroOnSight) (Variables|Default|GetisHeroHere))
    (Utilities|FlowControl|Sequence
      (:then_0
        (Transformation|SetActorRotation (Math|Rotator|FindLookatRotation (Transformation|GetActorLocation) (Transformation|GetActorLocation (Variables|Default|GetHeroCharRef)))))
      (:then_1
        (Utilities|FlowControl|DoOnce false
          (:Completed
            (Utilities|Time|SetTimerbyFunctionName 0 "Fire" (/ 1.0 (Variables|Default|GetShootPersecond)) true)))))))

(fn ConstructionScript)

(fn Fire
  (Game|SpawnActorfromClass "/Game/Enemy/Projetil/BP_ProjetilEnemy.BP_ProjetilEnemy_C" (Transformation|GetWorldTransform (Variables|Default|GetArrowProjetil)) "Undefined" "MultiplyWithRoot" 0 0))