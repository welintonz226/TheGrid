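; BP_ProjetilEnemyBoss is an enemy boss projectile that damages the player's hero on impact.
; On BeginPlay it sets a short life span and caches the player character as a BP_Herochar reference.
; On Hit it compares the other actor to that reference, calls HeroDamage with its Damage value on a match, and destroys itself whatever it struck.
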(event EventBeginPlay
  (Utilities|FlowControl|Sequence
    (:then_0
      (Actor|SetLifeSpan 2.0))
    (:then_1
      (bind _asbp_herochar (Utilities|Casting|CastToBP_Herochar (Game|GetPlayerCharacter 0)))
      (Variables|Default|SetHeroCharRef _asbp_herochar))))

(event Collision|EventHit
  (params (MyComp :type Primitive%20Component%20Object%20Reference) (Other :type Actor%20Object%20Reference) (OtherComp :type Primitive%20Component%20Object%20Reference) (bSelfMoved :type Boolean) (HitLocation :type Vector :default "0, 0, 0") (HitNormal :type Vector :default "0, 0, 0") (NormalImpulse :type Vector :default "0, 0, 0") (Hit :type Hit%20Result%20Structure%20%28by%20ref%29))
  (bind _herocharref (Variables|Default|GetHeroCharRef))
  ;[0.03646 0.03646 0.03646] Call function Damage no HeroChar
  (if (== Other _herocharref)
    (Default|HeroDamage _herocharref (Variables|Default|GetDamage))
    (Actor|DestroyActor)
    (else
      (Actor|DestroyActor))))

(fn ConstructionScript)